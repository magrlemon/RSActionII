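; T90 tank vehicle Blueprint that soldier characters can detect when they come near.
; The construction script and InitBP build both tracks from instanced static meshes, and InitBP also sets the main weapon's shell, feeds the tracks to the movement component, initializes the barrel and disables track physics.
; A detection sphere reports soldiers entering or leaving its range to the SoldierGameInstance through VehicleDetect.
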(event OnComponentBeginOverlap(SphereDetection)
  (params (OverlappedComponent :type Primitive%20Component%20Object%20Reference) (OtherActor :type Actor%20Object%20Reference) (OtherComp :type Primitive%20Component%20Object%20Reference) (OtherBodyIndex :type Integer) (bFromSweep :type Boolean) (SweepResult :type Hit%20Result%20Structure%20%28by%20ref%29))
  (bind _assoldier_character (Utilities|Casting|CastToSoldierCharacter OtherActor))
  (Utilities|IsValid _assoldier_character
    (:Is%20Valid
      (bind _assoldier_game_instance (Utilities|Casting|CastToSoldierGameInstance (Game|GetGameInstance)))
      (Class|SoldierGameInstance|VehicleDetect _assoldier_game_instance true self _assoldier_character))))

(event OnComponentEndOverlap(SphereDetection)
  (params (OverlappedComponent :type Primitive%20Component%20Object%20Reference) (OtherActor :type Actor%20Object%20Reference) (OtherComp :type Primitive%20Component%20Object%20Reference) (OtherBodyIndex :type Integer))
  (bind _assoldier_character (Utilities|Casting|CastToSoldierCharacter OtherActor))
  (Utilities|IsValid _assoldier_character
    (:Is%20Valid
      (bind _assoldier_game_instance (Utilities|Casting|CastToSoldierGameInstance (Game|GetGameInstance)))
      (Class|SoldierGameInstance|VehicleDetect _assoldier_game_instance false self _assoldier_character))))

(event EventBeginPlay)

(event Collision|EventActorBeginOverlap
  (params (OtherActor :type Actor%20Object%20Reference)))

(event EventTick
  (params (DeltaSeconds :type Float%20%28single-precision%29)))

(event EventInitBP
  (Utilities|FlowControl|Sequence
    (:then_0
      (Class|TankMainWeaponComponent|ChangeShellType (Variables|Default|GetMainWeaponComponent) "/Game/T90/BluePrints/TankProjectile_BP.TankProjectile_BP_C"))
    (:then_1
      (Class|TrackComponent|BuildTrack (Variables|Default|GetTrackLL) (Variables|Default|GetInstancedStaticMeshLL)))
    (:then_2
      (Class|TrackComponent|BuildTrack (Variables|Default|GetTrackLR) (Variables|Default|GetInstancedStaticMeshR)))
    (:then_3
      (Class|TankMovementComponent|Init (Variables|Default|GetMovementComponent) (Variables|Default|GetTrackLL) (Variables|Default|GetTrackLR)))
    (:then_4
      (Class|Tank|InitBarrel (Variables|Default|Getpaoguan)))
    (:then_5
      (Class|Tank|EnablePhysicMass false))))

(event EventEnablePhysicMass
  (params (enable :type Boolean))
  (Physics|SetSimulatePhysics (Variables|Default|GetTrackLR) enable)
  (Physics|SetSimulatePhysics (Variables|Default|GetTrackLL) enable))

(fn ConstructionScript
  (Class|TrackComponent|BuildTrack (Variables|Default|GetTrackLR) (Variables|Default|GetInstancedStaticMeshR))
  (Class|TrackComponent|BuildTrack (Variables|Default|GetTrackLL) (Variables|Default|GetInstancedStaticMeshLL)))